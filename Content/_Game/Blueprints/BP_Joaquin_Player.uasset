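; BP_Joaquin_Player is the player Blueprint for Joaquín, handling movement, camera look and jumping.
; Forward and right axis inputs move him relative to the control rotation's yaw only, and are ignored while the Combate (combat) flag is set.
; Look axes feed controller pitch and yaw, and Space Bar triggers Jump, neither gated by that flag.
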(event `InputAxis|MoveForward`
  (params (AxisValue :type "Float (single-precision)"))
  (if (not (`self.combate`))
    ; Movimiento AWSD Joaquín
    (`self.AddMovementInput` (`KismetMathLibrary.GetForwardVector` (`KismetMathLibrary.MakeRotator` 0.0 0.0 (.yaw (`self.GetControlRotation`)))) AxisValue)))

(event `InputAxis|LookUp`
  (params (AxisValue :type "Float (single-precision)"))
  ; Movimiento cámara Joaquín
  (`self.AddControllerPitchInput` AxisValue))

(event `InputAxis|LookRight`
  (params (AxisValue :type "Float (single-precision)"))
  ; Movimiento cámara Joaquín
  (`self.AddControllerYawInput` AxisValue))

(event `InputAxis|MoveRight`
  (params (AxisValue :type "Float (single-precision)"))
  ; Movimiento AWSD Joaquín
  (if (not (`self.combate`))
    (`self.AddMovementInput` (`KismetMathLibrary.GetRightVector` (`KismetMathLibrary.MakeRotator` 0.0 0.0 (.yaw (`self.GetControlRotation`)))) AxisValue)))

(event `Key|SpaceBar`
  (params (Key :type "Key Structure"))
  ; Salto Joaquín
  (:`Pressed`
    (`self.Jump`)))

(fn `UserConstructionScript`)